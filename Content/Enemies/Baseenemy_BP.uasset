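; Base enemy pawn drawn as a Doom-style directional Paper2D flipbook sprite, with health, melee and ranged attacks, and a death sequence.
; Each tick derives an idle, moving or attack state, then picks and rotates a flipbook by the player's angle and side relative to the enemy's facing.
; Sight and damage set the blackboard's canseeplayer key; death stops the AI brain, plays death and corpse flipbooks, then destroys the actor.
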(event `self.ReceiveTick`
  (params (DeltaSeconds :type "Float (single-precision)"))
  (bind _returnvalue (`KismetMathLibrary.Normal` (- (`self.K2_GetActorLocation` (`GameplayStatics.GetPlayerCharacter` 0)) (`self.K2_GetActorLocation`))))
  (if (> (`KismetMathLibrary.VSize` (`MovementComponent.Velocity` (`self.CharacterMovement`))) 0.0)
    (if (`self.isattacking`)
      (switch `/Game/Enemies/AttackingState` (`self.attackstate`)
        (:`NewEnumerator0`
          (set `self.enemystate` "NewEnumerator2"))
        (:`NewEnumerator1`
          (set `self.enemystate` "NewEnumerator3")))
      (else
        (set `self.enemystate` "NewEnumerator1")))
    (elif (`self.isattacking`)
      (switch `/Game/Enemies/AttackingState` (`self.attackstate`)
        (:`NewEnumerator0`
          (set `self.enemystate` "NewEnumerator2"))
        (:`NewEnumerator1`
          (set `self.enemystate` "NewEnumerator3")))
      (else
        (set `self.enemystate` "NewEnumerator0"))))
  (if (`self.isdead`)
    (`self.Handle death`)
    (else
      (if (`self.canseeplayer`)
        (`self.Rotatetowardsplayer`))
      (set `self.degrees` (`KismetMathLibrary.DegAcos` (`KismetMathLibrary.Dot_VectorVector` (`self.GetActorForwardVector`) _returnvalue)))
      (if (< (`KismetMathLibrary.Dot_VectorVector` (`self.GetActorRightVector`) _returnvalue) 0.0)
        (`/Engine/EditorBlueprintResources/StandardMacros.CompareFloat` (`self.degrees`) 180.0
          (:`>`
            (`SceneComponent.K2_SetRelativeRotation` (`self.PaperFlipbook`) (struct :`Yaw` -90.0) false false :!label _label)
            (`PaperFlipbookComponent.SetFlipbook` (`self.PaperFlipbook`) (`|GetArrayItem` (select `/Game/Enemies/Enemystate` (`self.enemystate`) :`NewEnumerator0` (`self.flipbooksIdle`) :`NewEnumerator1` (`self.flipbooksmoving`) :`NewEnumerator2` (`self.flipbooksmeleeattack`) :`NewEnumerator3` (`self.flipbooksrangeattack`)))))
          (:`==`
            (goto _label))
          (:`<`
            (`/Engine/EditorBlueprintResources/StandardMacros.CompareFloat` (`self.degrees`) 135.0
              (:`>`
                (`SceneComponent.K2_SetRelativeRotation` (`self.PaperFlipbook`) (struct :`Yaw` 135.0) false false :!label _label_2)
                (`PaperFlipbookComponent.SetFlipbook` (`self.PaperFlipbook`) (`|GetArrayItem` (select `/Game/Enemies/Enemystate` (`self.enemystate`) :`NewEnumerator0` (`self.flipbooksIdle`) :`NewEnumerator1` (`self.flipbooksmoving`) :`NewEnumerator2` (`self.flipbooksmeleeattack`) :`NewEnumerator3` (`self.flipbooksrangeattack`)) 3)))
              (:`==`
                (goto _label_2))
              (:`<`
                (`/Engine/EditorBlueprintResources/StandardMacros.CompareFloat` (`self.degrees`) 90.0
                  (:`>`
                    (`SceneComponent.K2_SetRelativeRotation` (`self.PaperFlipbook`) (struct :`Yaw` 180.0) false false :!label _label_3)
                    (`PaperFlipbookComponent.SetFlipbook` (`self.PaperFlipbook`) (`|GetArrayItem` (select `/Game/Enemies/Enemystate` (`self.enemystate`) :`NewEnumerator0` (`self.flipbooksIdle`) :`NewEnumerator1` (`self.flipbooksmoving`) :`NewEnumerator2` (`self.flipbooksmeleeattack`) :`NewEnumerator3` (`self.flipbooksrangeattack`)) 2)))
                  (:`==`
                    (goto _label_3))
                  (:`<`
                    (`/Engine/EditorBlueprintResources/StandardMacros.CompareFloat` (`self.degrees`) 45.0
                      (:`>`
                        _)
                      (:`==`
                        _)
                      (:`<`
                        (goto _label)))
                    (`SceneComponent.K2_SetRelativeRotation` (`self.PaperFlipbook`) (struct :`Yaw` 45.0) false false)
                    (`PaperFlipbookComponent.SetFlipbook` (`self.PaperFlipbook`) (`|GetArrayItem` (select `/Game/Enemies/Enemystate` (`self.enemystate`) :`NewEnumerator0` (`self.flipbooksIdle`) :`NewEnumerator1` (`self.flipbooksmoving`) :`NewEnumerator2` (`self.flipbooksmeleeattack`) :`NewEnumerator3` (`self.flipbooksrangeattack`)) 1))))))))
        (else
          (`/Engine/EditorBlueprintResources/StandardMacros.CompareFloat` (`self.degrees`) 180.0
            (:`>`
              (`SceneComponent.K2_SetRelativeRotation` (`self.PaperFlipbook`) (struct :`Yaw` -45.0) false false :!label _label_4)
              (`PaperFlipbookComponent.SetFlipbook` (`self.PaperFlipbook`) (`|GetArrayItem` (select `/Game/Enemies/Enemystate` (`self.enemystate`) :`NewEnumerator0` (`self.flipbooksIdle`) :`NewEnumerator1` (`self.flipbooksmoving`) :`NewEnumerator2` (`self.flipbooksmeleeattack`) :`NewEnumerator3` (`self.flipbooksrangeattack`)) 1)))
            (:`==`
              (goto _label_4))
            (:`<`
              (`/Engine/EditorBlueprintResources/StandardMacros.CompareFloat` (`self.degrees`) 135.0
                (:`>`
                  (`SceneComponent.K2_SetRelativeRotation` (`self.PaperFlipbook`) (struct :`Yaw` 90.0) false false :!label _label_5)
                  (`PaperFlipbookComponent.SetFlipbook` (`self.PaperFlipbook`) (`|GetArrayItem` (select `/Game/Enemies/Enemystate` (`self.enemystate`) :`NewEnumerator0` (`self.flipbooksIdle`) :`NewEnumerator1` (`self.flipbooksmoving`) :`NewEnumerator2` (`self.flipbooksmeleeattack`) :`NewEnumerator3` (`self.flipbooksrangeattack`)) 4)))
                (:`==`
                  (goto _label_5))
                (:`<`
                  (`/Engine/EditorBlueprintResources/StandardMacros.CompareFloat` (`self.degrees`) 90.0
                    (:`>`
                      (`SceneComponent.K2_SetRelativeRotation` (`self.PaperFlipbook`) (struct :`Yaw` 45.0) false false :!label _label_6)
                      (`PaperFlipbookComponent.SetFlipbook` (`self.PaperFlipbook`) (`|GetArrayItem` (select `/Game/Enemies/Enemystate` (`self.enemystate`) :`NewEnumerator0` (`self.flipbooksIdle`) :`NewEnumerator1` (`self.flipbooksmoving`) :`NewEnumerator2` (`self.flipbooksmeleeattack`) :`NewEnumerator3` (`self.flipbooksrangeattack`)) 5)))
                    (:`==`
                      (goto _label_6))
                    (:`<`
                      (`/Engine/EditorBlueprintResources/StandardMacros.CompareFloat` (`self.degrees`) 45.0
                        (:`>`
                          _)
                        (:`==`
                          _)
                        (:`<`
                          (goto _label_4)))
                      (`SceneComponent.K2_SetRelativeRotation` :`self` (`self.PaperFlipbook`))
                      (`PaperFlipbookComponent.SetFlipbook` (`self.PaperFlipbook`) (`|GetArrayItem` (select `/Game/Enemies/Enemystate` (`self.enemystate`) :`NewEnumerator0` (`self.flipbooksIdle`) :`NewEnumerator1` (`self.flipbooksmoving`) :`NewEnumerator2` (`self.flipbooksmeleeattack`) :`NewEnumerator3` (`self.flipbooksrangeattack`)) 6)))))))))))))

(event `self.ReceiveAnyDamage`
  (params (Damage :type "Float (single-precision)") (DamageType :type "DamageType Object Reference") (InstigatedBy :type "Controller Object Reference") (DamageCauser :type "Actor Object Reference"))
  ;[1 1 1] Handle enemy damage
  (bind _output_get (set `self.health` (- (`self.health`) Damage)))
  (if (<= _output_get 0.0)
    (set `self.isdead` true)
    (else
      (`self.playsoundenemy` "/Game/Sounds/enemydamaged.enemydamaged")
      (set `self.canseeplayer` true)
      (`BlackboardComponent.SetValueAsBool` (`AIBlueprintHelperLibrary.GetBlackboard` null) "canseeplayer" true))))

(event `playsoundenemy`
  (params (Sound :type "SoundBase Object Reference"))
  (bind _output_get (set `self.Sound` Sound))
  (`GameplayStatics.PlaySoundAtLocation` _output_get (`self.K2_GetActorLocation`) (struct) 1.0 1.0 0.0 null null null null))

(event `Handle death`
  (bind _paperflipbook (`self.PaperFlipbook`))
  (bind (_returnvalue_roll _returnvalue_pitch _returnvalue_yaw) (`KismetMathLibrary.BreakRotator` (`KismetMathLibrary.FindLookAtRotation` (`self.K2_GetActorLocation`) (`self.K2_GetActorLocation` (`GameplayStatics.GetPlayerCharacter` 0)))))
  ;[1 1 1] Handle enemy death system
  (`self.K2_SetActorRotation` (`KismetMathLibrary.MakeRotator` 0.0 0.0 _returnvalue_yaw))
  (`/Engine/EditorBlueprintResources/StandardMacros.DoOnce` false
    (:`Completed`
      (`BrainComponent.StopLogic` (`AIController.BrainComponent` (`AIBlueprintHelperLibrary.GetAIController` self)) "isdead")
      (`CharacterMovementComponent.SetMovementMode` (`self.CharacterMovement`) "MOVE_Flying" 0)
      (`PrimitiveComponent.SetCollisionEnabled` (`self.CapsuleComponent`) "NoCollision")
      (`ActorComponent.Deactivate` (`self.CharacterMovement`))
      (`self.playsoundenemy` "/Game/Sounds/enemydeath.enemydeath")
      (`SceneComponent.K2_SetRelativeRotation` _paperflipbook (struct :`Yaw` -90.0) false false)
      (`PaperFlipbookComponent.SetFlipbook` _paperflipbook (`self.enemydeathflipbook`))
      (`KismetSystemLibrary.Delay` (- (`PaperFlipbookComponent.GetFlipbookLength` (`self.PaperFlipbook`)) 0.2))
      (`self.K2_AddActorLocalOffset` (0.0 0.0 -30.0))
      (`PaperFlipbookComponent.SetFlipbook` (`self.PaperFlipbook`) (`self.enemybodyflipbook`))
      (`KismetSystemLibrary.Delay` 4.0)
      (`self.K2_DestroyActor`))))

(event `Rotatetowardsplayer`
  ;[1 1 1] Handle enemy rotation
  (`self.K2_SetActorRotation` (`KismetMathLibrary.RInterpTo` (`self.K2_GetActorRotation`) (`KismetMathLibrary.FindLookAtRotation` (`self.K2_GetActorLocation`) (`self.K2_GetActorLocation` (`GameplayStatics.GetPlayerCharacter` 0))) (`GameplayStatics.GetWorldDeltaSeconds`) (`self.rotationspeed`))))

(event `self.PawnSensing.OnSeePawn`
  (params (Pawn :type "Pawn Object Reference"))
  ;[1 1 1] Handle enemy vision
  (cast `/Game/FirstPerson/Blueprints/BP_FirstPersonCharacter` Pawn)
  (set `self.canseeplayer` true)
  (`BlackboardComponent.SetValueAsBool` (`AIBlueprintHelperLibrary.GetBlackboard` null) "canseeplayer" true)
  (`KismetSystemLibrary.RetriggerableDelay` 0.7)
  (set `self.canseeplayer` false)
  (`BlackboardComponent.SetValueAsBool` (`AIBlueprintHelperLibrary.GetBlackboard` null) "canseeplayer" false))

(event `Meleeattack`
  (bind _returnvalue (`self.K2_GetActorLocation`))
  ;[1 1 1] Attack system
  ;;[1 0 0] Melee attack
  (set `self.isattacking` true)
  (set `self.attackstate` "NewEnumerator0")
  (bind _outhit (`KismetSystemLibrary.LineTraceSingleForObjects` _returnvalue (+ _returnvalue (* (`self.GetActorForwardVector`) 150.0)) (`|MakeArray` "ObjectTypeQuery3" :!type "EObjectTypeQuery Enum") false (`|MakeArray` self :!type "Actor Object Reference")))
  (bind (_bblockinghit _binitialoverlap _time _distance _location _impactpoint _normal _impactnormal _physmat _hitactor) (`GameplayStatics.BreakHitResult` _outhit))
  (if (== _hitactor (`GameplayStatics.GetPlayerCharacter` 0))
    (`GameplayStatics.ApplyDamage` _hitactor (`self.enemydamage`)))
  (`KismetSystemLibrary.RetriggerableDelay` (+ (`self.Meleerate`) 0.1))
  (set `self.isattacking` false))

(event `Spawnprojectile`
  ;[1 1 1] Attack system
  ;;[1 0 0] Range attack
  (set `self.isattacking` true)
  (set `self.attackstate` "NewEnumerator1")
  (`MovementComponent.StopMovementImmediately` (`self.CharacterMovement`))
  (`|SpawnActorFromClass` (`self.enemyprojectile`) (`SceneComponent.K2_GetComponentToWorld` (`self.projectilespawn`)) "Undefined" "MultiplyWithRoot" null (`self.Projectilespeed`) (`self.Projectiledamage`) null)
  (set `self.Sound` "/Game/Sounds/enemyprojectile.enemyprojectile")
  (`self.playsoundenemy` null)
  (`KismetSystemLibrary.RetriggerableDelay` (+ (`self.Firerate`) 0.1))
  (set `self.isattacking` false))

(fn `UserConstructionScript`)