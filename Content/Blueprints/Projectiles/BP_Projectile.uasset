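; Projectile actor with a Paper2D flipbook that deals damage on impact and plays a destruction animation.
; The construction script sets initial and max movement speed from one variable.
; Hit damages any actor, while Sphere overlap ignores the first player's character and also stops movement.
; Both then share a sequence that rescales the flipbook, plays a sound, swaps to the destroyed flipbook and destroys the actor after its length.
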(event `playprojectile sound`
  (`GameplayStatics.PlaySoundAtLocation` (`self.Sound`) (`self.K2_GetActorLocation`) (struct) 1.0 1.0 0.0 null null null null))

(event `self.ReceiveHit`
  (params (MyComp :type "PrimitiveComponent Object Reference") (Other :type "Actor Object Reference") (OtherComp :type "PrimitiveComponent Object Reference") (bSelfMoved :type Boolean) (HitLocation :type "Vector Structure") (HitNormal :type "Vector Structure") (NormalImpulse :type "Vector Structure") (Hit :type "HitResult Structure (by ref)"))
  (bind _paperflipbook (`self.PaperFlipbook`))
  (`GameplayStatics.ApplyDamage` Other (`self.projectiledamage`))
  (`SceneComponent.SetWorldScale3D` _paperflipbook (`self.destroyedscale`) :!label _label)
  (`self.playprojectile sound`)
  (`PaperFlipbookComponent.SetFlipbook` _paperflipbook (`self.destroyedprojectile`))
  (`KismetSystemLibrary.Delay` (`PaperFlipbookComponent.GetFlipbookLength` _paperflipbook))
  (`self.K2_DestroyActor`))

(event `self.Sphere.OnComponentBeginOverlap`
  (params (OverlappedComponent :type "PrimitiveComponent Object Reference") (OtherActor :type "Actor Object Reference") (OtherComp :type "PrimitiveComponent Object Reference") (OtherBodyIndex :type Integer) (bFromSweep :type Boolean) (SweepResult :type "HitResult Structure (by ref)"))
  (if (not (== OtherActor (`GameplayStatics.GetPlayerCharacter` 0)))
    (`GameplayStatics.ApplyDamage` OtherActor (`self.projectiledamage`))
    (`MovementComponent.StopMovementImmediately` (`self.ProjectileMovement`))
    (goto _label)))

(fn `UserConstructionScript`
  (bind _projectilemovement (`self.ProjectileMovement`))
  (bind _projectilespeed (`self.projectilespeed`))
  (set `ProjectileMovementComponent.InitialSpeed` _projectilespeed _projectilemovement)
  (set `ProjectileMovementComponent.MaxSpeed` _projectilespeed _projectilemovement))