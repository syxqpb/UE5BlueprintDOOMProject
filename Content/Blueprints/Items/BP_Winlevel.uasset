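; BP_Winlevel is a level-win trigger item that ends in a win screen when the first-person player reaches it.
; Each Tick it yaws to face the player character.
; The first Box overlap by BP_FirstPersonCharacter, gated by DoOnce, plays the win sound at the actor's location through a custom event.
; It then creates a WinGame widget, passing it the Level value, and adds it to the viewport.
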(event `self.ReceiveTick`
  (params (DeltaSeconds :type "Float (single-precision)"))
  (bind (_returnvalue_roll _returnvalue_pitch _returnvalue_yaw) (`KismetMathLibrary.BreakRotator` (`KismetMathLibrary.FindLookAtRotation` (`self.K2_GetActorLocation`) (`self.K2_GetActorLocation` (`GameplayStatics.GetPlayerCharacter` 0)))))
  (`self.K2_SetActorRotation` (`KismetMathLibrary.MakeRotator` 0.0 0.0 _returnvalue_yaw)))

(event `self.Box.OnComponentBeginOverlap`
  (params (OverlappedComponent :type "PrimitiveComponent Object Reference") (OtherActor :type "Actor Object Reference") (OtherComp :type "PrimitiveComponent Object Reference") (OtherBodyIndex :type Integer) (bFromSweep :type Boolean) (SweepResult :type "HitResult Structure (by ref)"))
  (cast `/Game/FirstPerson/Blueprints/BP_FirstPersonCharacter` OtherActor)
  (`/Engine/EditorBlueprintResources/StandardMacros.DoOnce` false
    (:`Completed`
      (`self.playsoundwinlevel` "/Game/Sounds/wingame.wingame")
      (bind _returnvalue (`|CreateWidget` "/Game/Blueprints/UI/WinGame.WinGame_C" null (`self.Level`)))
      (`UserWidget.AddToViewport` _returnvalue 0))))

(event `playsoundwinlevel`
  (params (Sound :type "SoundBase Object Reference"))
  (set `self.Sound` Sound)
  (`GameplayStatics.PlaySoundAtLocation` (`self.Sound`) (`self.K2_GetActorLocation`) (struct) 1.0 1.0 0.0 null null null null))

(fn `UserConstructionScript`)