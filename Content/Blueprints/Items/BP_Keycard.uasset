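; Keycard pickup actor shown as a Paper2D sprite, with blue, orange and red variants chosen by the Keycard enum.
; The construction script sets the sprite for the chosen color, and Tick yaws the actor to face the player like a billboard.
; When the first-person character overlaps the box, it plays a pickup sound, sets that character's matching keycard flag, updates the HUD and destroys itself.
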(event `self.ReceiveTick`
  (params (DeltaSeconds :type "Float (single-precision)"))
  (bind (_returnvalue_roll _returnvalue_pitch _returnvalue_yaw) (`KismetMathLibrary.BreakRotator` (`KismetMathLibrary.FindLookAtRotation` (`self.K2_GetActorLocation`) (`self.K2_GetActorLocation` (`GameplayStatics.GetPlayerCharacter` 0)))))
  (`self.K2_SetActorRotation` (`KismetMathLibrary.MakeRotator` 0.0 0.0 _returnvalue_yaw)))

(event `self.Box.OnComponentBeginOverlap`
  (params (OverlappedComponent :type "PrimitiveComponent Object Reference") (OtherActor :type "Actor Object Reference") (OtherComp :type "PrimitiveComponent Object Reference") (OtherBodyIndex :type Integer) (bFromSweep :type Boolean) (SweepResult :type "HitResult Structure (by ref)"))
  (bind _firstperoncharacterref (`self.firstperoncharacterref`))
  (bind _firstperoncharacterref_2 (`self.firstperoncharacterref`))
  (bind _firstperoncharacterref_3 (`self.firstperoncharacterref`))
  (bind _asbp_first_person_character (cast `/Game/FirstPerson/Blueprints/BP_FirstPersonCharacter` OtherActor))
  (set `self.firstperoncharacterref` _asbp_first_person_character)
  (`self.playsound` "/Game/Sounds/pickup.pickup")
  (switch `/Game/Blueprints/Items/Keycard` (`self.keycard`)
    (:`NewEnumerator0`
      (set `/Game/FirstPerson/Blueprints/BP_FirstPersonCharacter.bluekeycard?` true _firstperoncharacterref_2)
      (`/Game/Blueprints/UI/PlayerHUD.findbluecardkey` (`/Game/FirstPerson/Blueprints/BP_FirstPersonCharacter.playerhud` _firstperoncharacterref_2))
      (`self.K2_DestroyActor`))
    (:`NewEnumerator1`
      (set `/Game/FirstPerson/Blueprints/BP_FirstPersonCharacter.orangekeycard?` true _firstperoncharacterref_3)
      (`/Game/Blueprints/UI/PlayerHUD.findorangekeycard` (`/Game/FirstPerson/Blueprints/BP_FirstPersonCharacter.playerhud` _firstperoncharacterref_3))
      (`self.K2_DestroyActor`))
    (:`NewEnumerator2`
      (set `/Game/FirstPerson/Blueprints/BP_FirstPersonCharacter.redkeycard?` true _firstperoncharacterref)
      (`/Game/Blueprints/UI/PlayerHUD.findredkeycard` (`/Game/FirstPerson/Blueprints/BP_FirstPersonCharacter.playerhud` _firstperoncharacterref))
      (`self.K2_DestroyActor`))))

(event `playsound`
  (params (Sound :type "SoundBase Object Reference"))
  (bind _output_get (set `self.Sound` Sound))
  (`GameplayStatics.PlaySoundAtLocation` _output_get (`self.K2_GetActorLocation`) (struct) 1.0 1.0 0.0 null null null null))

(fn `UserConstructionScript`
  (switch `/Game/Blueprints/Items/Keycard` (`self.keycard`)
    (:`NewEnumerator0`
      (`PaperSpriteComponent.SetSprite` (`self.PaperSprite`) "/Game/Spites/Items/bluekey_Sprite.bluekey_Sprite"))
    (:`NewEnumerator1`
      (`PaperSpriteComponent.SetSprite` (`self.PaperSprite`) "/Game/Spites/Items/orangekey_Sprite.orangekey_Sprite"))
    (:`NewEnumerator2`
      (`PaperSpriteComponent.SetSprite` (`self.PaperSprite`) "/Game/Spites/Items/redkey_Sprite.redkey_Sprite"))))