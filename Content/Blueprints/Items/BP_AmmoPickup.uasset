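; Ammo pickup actor that adds bullets, shells, rockets or cells to the first-person character when it overlaps the box.
; The Ammotype enum picks the sprite in the construction script, and Tick yaws the billboard toward the player.
; On overlap it plays a sound once, adds the clamped amount, refreshes the player HUD, spawns an ammo HUD widget and destroys itself.
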(event `self.ReceiveTick`
  (params (DeltaSeconds :type "Float (single-precision)"))
  (bind (_returnvalue_roll _returnvalue_pitch _returnvalue_yaw) (`KismetMathLibrary.BreakRotator` (`KismetMathLibrary.FindLookAtRotation` (`self.K2_GetActorLocation`) (`self.K2_GetActorLocation` (`GameplayStatics.GetPlayerCharacter` 0)))))
  (`self.K2_SetActorRotation` (`KismetMathLibrary.MakeRotator` 0.0 0.0 _returnvalue_yaw)))

(event `self.Box.OnComponentBeginOverlap`
  (params (OverlappedComponent :type "PrimitiveComponent Object Reference") (OtherActor :type "Actor Object Reference") (OtherComp :type "PrimitiveComponent Object Reference") (OtherBodyIndex :type Integer) (bFromSweep :type Boolean) (SweepResult :type "HitResult Structure (by ref)"))
  (bind _as_bp_first_person_character (`self.As BP First Person Character`))
  (bind _as_bp_first_person_character_2 (`self.As BP First Person Character`))
  (bind _as_bp_first_person_character_3 (`self.As BP First Person Character`))
  (bind _as_bp_first_person_character_4 (`self.As BP First Person Character`))
  (bind _as_bp_first_person_character_5 (`self.As BP First Person Character`))
  (bind _as_bp_first_person_character_6 (`self.As BP First Person Character`))
  (bind _as_bp_first_person_character_7 (`self.As BP First Person Character`))
  (bind _as_bp_first_person_character_8 (`self.As BP First Person Character`))
  (bind _asbp_first_person_character (cast `/Game/FirstPerson/Blueprints/BP_FirstPersonCharacter` OtherActor))
  (set `self.As BP First Person Character` _asbp_first_person_character)
  (`/Engine/EditorBlueprintResources/StandardMacros.DoOnce` false
    (:`Completed`
      (`self.playsoundpickup` "/Game/Sounds/pickup.pickup")
      (switch `/Game/Blueprints/Items/Ammotype` (`self.ammotype`)
        (:`NewEnumerator0`
          (set `/Game/FirstPerson/Blueprints/BP_FirstPersonCharacter.bullet` (`KismetMathLibrary.Clamp` (+ (`/Game/FirstPerson/Blueprints/BP_FirstPersonCharacter.bullet` _as_bp_first_person_character_8) (`self.ammotogive`)) 0 (`/Game/FirstPerson/Blueprints/BP_FirstPersonCharacter.maxbullet` _as_bp_first_person_character_8)) _as_bp_first_person_character_2)
          (`/Game/Blueprints/UI/PlayerHUD.Updatebulletammo` (`/Game/FirstPerson/Blueprints/BP_FirstPersonCharacter.playerhud` _as_bp_first_person_character_2))
          (bind _returnvalue (`|CreateWidget` "/Game/Blueprints/UI/PlayerAmmoHUD.PlayerAmmoHUD_C"))
          (`UserWidget.AddToViewport` _returnvalue 0)
          (`self.K2_DestroyActor`))
        (:`NewEnumerator2`
          (set `/Game/FirstPerson/Blueprints/BP_FirstPersonCharacter.shell` (`KismetMathLibrary.Clamp` (+ (`/Game/FirstPerson/Blueprints/BP_FirstPersonCharacter.shell` _as_bp_first_person_character_3) (`self.ammotogive`)) 0 (`/Game/FirstPerson/Blueprints/BP_FirstPersonCharacter.maxshell` _as_bp_first_person_character_3)) _as_bp_first_person_character_4)
          (`/Game/Blueprints/UI/PlayerHUD.Updateshellammo` (`/Game/FirstPerson/Blueprints/BP_FirstPersonCharacter.playerhud` _as_bp_first_person_character_4))
          (bind _returnvalue_2 (`|CreateWidget` "/Game/Blueprints/UI/PlayerAmmoHUD.PlayerAmmoHUD_C"))
          (`UserWidget.AddToViewport` _returnvalue_2 0)
          (`self.K2_DestroyActor`))
        (:`NewEnumerator1`
          (set `/Game/FirstPerson/Blueprints/BP_FirstPersonCharacter.rock` (`KismetMathLibrary.Clamp` (+ (`/Game/FirstPerson/Blueprints/BP_FirstPersonCharacter.rock` _as_bp_first_person_character_5) (`self.ammotogive`)) 0 (`/Game/FirstPerson/Blueprints/BP_FirstPersonCharacter.maxrock` _as_bp_first_person_character_5)) _as_bp_first_person_character_6)
          (`/Game/Blueprints/UI/PlayerHUD.Updaterockammo` (`/Game/FirstPerson/Blueprints/BP_FirstPersonCharacter.playerhud` _as_bp_first_person_character_6))
          (bind _returnvalue_3 (`|CreateWidget` "/Game/Blueprints/UI/PlayerAmmoHUD.PlayerAmmoHUD_C"))
          (`UserWidget.AddToViewport` _returnvalue_3 0)
          (`self.K2_DestroyActor`))
        (:`NewEnumerator3`
          (set `/Game/FirstPerson/Blueprints/BP_FirstPersonCharacter.cell` (`KismetMathLibrary.Clamp` (+ (`/Game/FirstPerson/Blueprints/BP_FirstPersonCharacter.cell` _as_bp_first_person_character) (`self.ammotogive`)) 0 (`/Game/FirstPerson/Blueprints/BP_FirstPersonCharacter.maxcell` _as_bp_first_person_character)) _as_bp_first_person_character_7)
          (`/Game/Blueprints/UI/PlayerHUD.UpdateCellammo` (`/Game/FirstPerson/Blueprints/BP_FirstPersonCharacter.playerhud` _as_bp_first_person_character_7))
          (bind _returnvalue_4 (`|CreateWidget` "/Game/Blueprints/UI/PlayerAmmoHUD.PlayerAmmoHUD_C"))
          (`UserWidget.AddToViewport` _returnvalue_4 0)
          (`self.K2_DestroyActor`))))))

(event `playsoundpickup`
  (params (Sound :type "SoundBase Object Reference"))
  (bind _output_get (set `self.Sound` Sound))
  (`GameplayStatics.PlaySoundAtLocation` _output_get (`self.K2_GetActorLocation`) (struct) 1.0 1.0 0.0 null null null null))

(fn `UserConstructionScript`
  (switch `/Game/Blueprints/Items/Ammotype` (`self.ammotype`)
    (:`NewEnumerator0`
      (`PaperSpriteComponent.SetSprite` (`self.PaperSprite`) "/Game/Spites/Items/NormalAmmo_Sprite.NormalAmmo_Sprite"))
    (:`NewEnumerator2`
      (`PaperSpriteComponent.SetSprite` (`self.PaperSprite`) "/Game/Spites/Items/Shotgun_Sprite.Shotgun_Sprite"))
    (:`NewEnumerator1`
      (`PaperSpriteComponent.SetSprite` (`self.PaperSprite`) "/Game/Spites/Items/Rocket_Sprite.Rocket_Sprite"))
    (:`NewEnumerator3`
      (`PaperSpriteComponent.SetSprite` (`self.PaperSprite`) "/Game/Spites/Items/cellammo_Sprite.cellammo_Sprite"))))