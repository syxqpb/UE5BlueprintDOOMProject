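; Base weapon actor for the first-person character, with empty shoot and stop events, presumably for child weapons to override.
; It offers hitscan fire, applying damage and spawning blood on "enemy"-tagged actors or a surface-aligned actor elsewhere, plus projectile fire passing speed and damage.
; An ammo type selects which player-held counter is checked or decremented, with decrements updating the HUD.
; A helper event plays the weapon sound at its location.
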(event `self.ReceiveBeginPlay`
  (bind _asbp_first_person_character (cast `/Game/FirstPerson/Blueprints/BP_FirstPersonCharacter` (`GameplayStatics.GetPlayerCharacter` 0)))
  (set `self.Playercharacterref` _asbp_first_person_character))

(event `ShootWeapon`)

(event `StopShooting`)

(event `Decreaseammo`
  (bind _playercharacterref (`self.Playercharacterref`))
  (bind _playercharacterref_2 (`self.Playercharacterref`))
  (bind _playercharacterref_3 (`self.Playercharacterref`))
  (bind _playercharacterref_4 (`self.Playercharacterref`))
  (switch `/Game/Blueprints/Weapons/Ammo` (`self.ammotype`)
    (:`NewEnumerator0`
      (`/Engine/EditorBlueprintResources/StandardMacros.DecrementInt` (`/Game/FirstPerson/Blueprints/BP_FirstPersonCharacter.bullet` _playercharacterref_2)
        (:`  `
          (`/Game/Blueprints/UI/PlayerHUD.Updatebulletammo` (`/Game/FirstPerson/Blueprints/BP_FirstPersonCharacter.playerhud` _playercharacterref_2)))))
    (:`NewEnumerator1`
      (`/Engine/EditorBlueprintResources/StandardMacros.DecrementInt` (`/Game/FirstPerson/Blueprints/BP_FirstPersonCharacter.shell` _playercharacterref_3)
        (:`  `
          (`/Game/Blueprints/UI/PlayerHUD.Updateshellammo` (`/Game/FirstPerson/Blueprints/BP_FirstPersonCharacter.playerhud` _playercharacterref_3)))))
    (:`NewEnumerator2`
      (`/Engine/EditorBlueprintResources/StandardMacros.DecrementInt` (`/Game/FirstPerson/Blueprints/BP_FirstPersonCharacter.rock` _playercharacterref_4)
        (:`  `
          (`/Game/Blueprints/UI/PlayerHUD.Updaterockammo` (`/Game/FirstPerson/Blueprints/BP_FirstPersonCharacter.playerhud` _playercharacterref_4)))))
    (:`NewEnumerator3`
      (`/Engine/EditorBlueprintResources/StandardMacros.DecrementInt` (`/Game/FirstPerson/Blueprints/BP_FirstPersonCharacter.cell` _playercharacterref)
        (:`  `
          (`/Game/Blueprints/UI/PlayerHUD.UpdateCellammo` (`/Game/FirstPerson/Blueprints/BP_FirstPersonCharacter.playerhud` _playercharacterref)))))))

(event `play weapon sound`
  (`GameplayStatics.PlaySoundAtLocation` (`self.Sound`) (`self.K2_GetActorLocation`) (struct) 1.0 1.0 0.0 null null null null))

(fn `Fireprojectile`
  (`|SpawnActorFromClass` (`self.projectile`) (`SceneComponent.K2_GetComponentToWorld` (`self.projectiletransform`)) "Undefined" "MultiplyWithRoot" null (`self.projectilespeed`) (`self.Weapondamage`) null))

(fn `Fireweapon`
  (bind _returnvalue (`SceneComponent.K2_GetComponentLocation` (`self.linetrace`)))
  (bind (_outhit _returnvalue_2) (`KismetSystemLibrary.LineTraceSingleForObjects` _returnvalue (+ _returnvalue (* (`KismetMathLibrary.GetForwardVector` (`SceneComponent.K2_GetComponentRotation` (`self.linetrace`))) (`self.Linetracedistance`))) (`|MakeArray` "ObjectTypeQuery1" "ObjectTypeQuery2" "ObjectTypeQuery3" :!type "EObjectTypeQuery Enum") false (`|MakeArray` self (`GameplayStatics.GetPlayerCharacter` 0) :!type "Actor Object Reference")))
  (if _returnvalue_2
    (bind (_bblockinghit _binitialoverlap _time _distance _location _impactpoint _normal _impactnormal _physmat _hitactor) (`GameplayStatics.BreakHitResult` _outhit))
    (`GameplayStatics.ApplyDamage` _hitactor (`self.Weapondamage`))
    (if (`self.ActorHasTag` _hitactor "enemy")
      (`|SpawnActorFromClass` "/Game/Enemies/Blood/Blood_BP.Blood_BP_C" (`KismetMathLibrary.MakeTransform` _location) "Undefined" "MultiplyWithRoot" null null)
      (else
        (`|SpawnActorFromClass` "/Game/Blueprints/Hit_BP.Hit_BP_C" (`KismetMathLibrary.MakeTransform` (- _location (0.0 0.0 -0.15)) (`KismetMathLibrary.ComposeRotators` (`KismetMathLibrary.Conv_VectorToRotator` _normal) (struct :`Yaw` -90.0))) "Undefined" "MultiplyWithRoot" null null)))))

(fn `Hasenoughammo?`
  (returns (Hasammo :type Boolean))
  (switch `/Game/Blueprints/Weapons/Ammo` (`self.ammotype`)
    (:`NewEnumerator0`
      (if (> (`/Game/FirstPerson/Blueprints/BP_FirstPersonCharacter.bullet` (`self.Playercharacterref`)) 0)
        (return true)
        (else
          (return false))))
    (:`NewEnumerator1`
      (if (> (`/Game/FirstPerson/Blueprints/BP_FirstPersonCharacter.shell` (`self.Playercharacterref`)) 0)
        (return true)
        (else
          (return false))))
    (:`NewEnumerator2`
      (if (> (`/Game/FirstPerson/Blueprints/BP_FirstPersonCharacter.rock` (`self.Playercharacterref`)) 0)
        (return true)
        (else
          (return false))))
    (:`NewEnumerator3`
      (if (> (`/Game/FirstPerson/Blueprints/BP_FirstPersonCharacter.cell` (`self.Playercharacterref`)) 0)
        (return true)
        (else
          (return false))))))

(fn `UserConstructionScript`)