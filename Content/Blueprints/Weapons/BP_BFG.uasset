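; BP_BFG is the BFG weapon, which overrides ShootWeapon to fire a projectile at a cost of 30 Cell ammo.
; A shot requires enough cells, then plays the sound and fire flipbook, waiting for the animation's length before launching the projectile.
; It then restores the idle flipbook, deducts the ammo and updates the player HUD.
; A DoOnce, reset after each shot, blocks refiring mid-sequence.
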(event `self.ShootWeapon`
  (bind _playercharacterref (`self.Playercharacterref`))
  (bind _weaponflipbook (`self.Weaponflipbook`))
  (if (>= (`/Game/FirstPerson/Blueprints/BP_FirstPersonCharacter.cell` (`self.Playercharacterref`)) 30)
    (`/Engine/EditorBlueprintResources/StandardMacros.DoOnce` false :!label _label
      (:`Completed`
        (`self.play weapon sound`)
        (`PaperFlipbookComponent.SetFlipbook` _weaponflipbook "/Game/Spites/Weapons/BFG/BFGFire.BFGFire")
        (`KismetSystemLibrary.Delay` (`PaperFlipbookComponent.GetFlipbookLength` _weaponflipbook))
        (`self.Fireprojectile`)
        (`PaperFlipbookComponent.SetFlipbook` (`self.Weaponflipbook`) "/Game/Spites/Weapons/BFG/BFGIdle.BFGIdle")
        (set `/Game/FirstPerson/Blueprints/BP_FirstPersonCharacter.cell` (- (`/Game/FirstPerson/Blueprints/BP_FirstPersonCharacter.cell` _playercharacterref) 30) _playercharacterref)
        (`/Game/Blueprints/UI/PlayerHUD.UpdateCellammo` (`/Game/FirstPerson/Blueprints/BP_FirstPersonCharacter.playerhud` _playercharacterref))
        (`self.RESETDOONCE`)))))

(event `RESETDOONCE`
  (goto _label :!via `Reset`))

(fn `UserConstructionScript`
  (`parent.UserConstructionScript`))