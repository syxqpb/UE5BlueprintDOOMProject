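; BP_Chainsaw is a chainsaw weapon that attacks continuously while shooting is active.
; ShootWeapon passes a DoOnce gate to start a looping timer, which repeatedly calls Fireweapon, plays the saw sound and sets the attack flipbook.
; StopShooting clears the timer, restores the idle flipbook and resets the gate, so repeated shoot calls cannot stack timers.
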(event `self.ReceiveTick`
  (params (DeltaSeconds :type "Float (single-precision)"))
  (`parent.ReceiveTick` DeltaSeconds))

(event `self.ShootWeapon`
  (`/Engine/EditorBlueprintResources/StandardMacros.DoOnce` false :!label _label
    (:`Completed`
      (bind _returnvalue (`KismetSystemLibrary.K2_SetTimerDelegate` (delegate `usechainsaw`) 0.23 true))
      (set `self.chainsawevent` _returnvalue))))

(event `resetchainsaw`
  (goto _label :!via `Reset`))

(event `usechainsaw`
  (`self.Fireweapon`)
  (set `self.Sound` "/Game/Spites/Weapons/Chainsaw/dssawful.dssawful")
  (`self.play weapon sound`)
  (`PaperFlipbookComponent.SetFlipbook` (`self.Weaponflipbook`) "/Game/Spites/Weapons/Chainsaw/Chainsawattack.Chainsawattack"))

(event `self.StopShooting`
  (`KismetSystemLibrary.K2_ClearAndInvalidateTimerHandle` (`self.chainsawevent`))
  (`PaperFlipbookComponent.SetFlipbook` (`self.Weaponflipbook`) "/Game/Spites/Weapons/Chainsaw/Chainsawidle.Chainsawidle")
  (`self.resetchainsaw`))

(fn `UserConstructionScript`
  (`parent.UserConstructionScript`))